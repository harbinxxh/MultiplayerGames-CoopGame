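; BP_CustomGunPlayer is a player Blueprint for the CustomGun challenge that equips a gun and handles firing input.
; On BeginPlay it spawns a BP_CustomGun it owns, stores it as CurrentWeapon, attaches it to the mesh's WeaponSocket and adds a crosshair widget to the viewport.
; Left mouse press and release cast CurrentWeapon to BP_CustomGun and call OnOpenFireEvent with true or false, leaving firing logic to the gun.
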(event EventBeginPlay
  (bind _returnvalue (Game|SpawnActorfromClass "/Game/Challenges/CustomGun/BP_CustomGun.BP_CustomGun_C" (Math|Transform|MakeTransform "0, 0, 0") "AlwaysSpawn" self 0))
  (Variables|Default|SetCurrentWeapon _returnvalue)
  (Transformation|AttachComponentToComponent _returnvalue (Variables|Character|GetMesh) "WeaponSocket" "SnapToTarget" "SnapToTarget" "SnapToTarget" true)
  (bind _returnvalue_2 (UserInterface|CreateWidget "/Game/UI/WBP_Crosshair.WBP_Crosshair_C"))
  (UserInterface|Viewport|AddtoViewport _returnvalue_2 0))

(event Input|MouseEvents|LeftMouseButton
  (params (Key :type Key%20Structure))
  (bind _currentweapon (Variables|Default|GetCurrentWeapon))
  (:Pressed
    (bind _asbp_custom_gun (Utilities|Casting|CastToBP_CustomGun _currentweapon))
    (Default|OnOpenFireEvent _asbp_custom_gun true))
  (:Released
    (bind _asbp_custom_gun_2 (Utilities|Casting|CastToBP_CustomGun _currentweapon))
    (Default|OnOpenFireEvent _asbp_custom_gun_2 false)))

(fn ConstructionScript)