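; BP_GrenadeProjectile is a timed grenade projectile for the grenade launcher challenge that explodes one second after spawning.
; BeginPlay waits on a fixed delay, then calls Explode, with no impact trigger in its graphs.
; Explode spawns a particle effect, applies radial damage credited to the instigator's controller, and destroys the actor.
; A debug sphere showing the damage radius is drawn after the DestroyActor call.
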(event Custom|Explode
  (bind _returnvalue (Transformation|GetActorLocation))
  (bind _damageradius (Variables|Default|GetDamageRadius))
  (Effects|SpawnEmitteratLocation "/Game/WeaponEffects/Explosion/P_Explosion.P_Explosion" _returnvalue)
  (Game|Damage|ApplyRadialDamage 1e+02 _returnvalue _damageradius 0 0 self (Game|GetInstigatorController) false "ECC_Visibility")
  (Actor|DestroyActor)
  (Rendering|Debug|DrawDebugSphere _returnvalue _damageradius 12 "(R=1.000000,G=0.909027,B=0.014317,A=1.000000)" 1.0 2.0))

(event EventBeginPlay
  (Utilities|FlowControl|Delay 1.0)
  (CallFunction|Explode))

(fn ConstructionScript)