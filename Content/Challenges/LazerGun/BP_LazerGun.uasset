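; Laser gun weapon that fires a particle beam along its owner's view while the fire flag is set.
; Tick starts the LazereGun loop once per press; it repeats every 0.2 seconds, line-tracing from the muzzle socket toward the eye-view target.
; Y-axis hit distance sizes nearby beams and spawns impacts, though the length parameter name there is None.
; Misses and far hits use fixed length; ApplyDamage has no target wired.
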(event Custom|OnOpenFireEvent
  (params (IsFire :type Boolean))
  (Variables|Default|SetIsFire IsFire))

(event Custom|CalcTargetEnd
  (bind _returnvalue (Components|GetOwner))
  (bind (_outlocation _outrotation) (Actor|GetActorEyesViewPoint _returnvalue))
  (bind _output_get (Variables|Default|SetTargetEnd (+ _outlocation (* (Math|Vector|GetForwardVector _outrotation) 10000))))
  (Development|PrintString (Utilities|String|ToString(Vector) _output_get)))

(event EventBeginPlay
  (Components|Activation|Deactivate (Variables|Default|GetLager_P)))

(event EventTick
  (params (DeltaSeconds :type Float%20%28single-precision%29))
  (if (Variables|Default|GetIsFire)
    (Utilities|FlowControl|DoOnce true :!label _label
      (:Completed
        (Utilities|LazereGun)))
    (else
      (Components|Activation|Deactivate (Variables|Default|GetLager_P))
      (goto _label Reset))))

(fn ConstructionScript)