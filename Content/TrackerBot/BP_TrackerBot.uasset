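; BP_TrackerBot is a tracker bot Blueprint that scales the volume of its audio component with its movement speed.
; Each Tick maps velocity magnitude through a clamped range to the volume multiplier, so faster movement sounds louder.
; Disconnected experimental nodes show three navigation approaches: moving to a fixed location, moving to the player, and drawing debug spheres along a synchronous path to the player.
; None of these navigation chains execute.
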(event EventBeginPlay)

(event EventTick
  (params (DeltaSeconds :type Float%20%28single-precision%29))
  ;[1 1 1] I'd like to make this volume change based on the current velocity. 我想让声音的变化是基于当前的速度而改变。
  (Audio|Components|Audio|SetVolumeMultiplier (Variables|Default|GetAudioComp) (Math|Float|MapRangeClamped (Math|Vector|VectorLength (Transformation|GetVelocity)) 1e+01 1e+03 0.1 2.0) :!class /Script/Engine.AudioComponent))

(fn ConstructionScript)