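; BP_TrackerBot is a tracker bot Blueprint holding three numbered navigation experiments, none connected to an event, so it currently does nothing at runtime.
; The disconnected snippets move its AI controller to the world origin with Simple Move to Location or toward player 0 with Simple Move to Actor, noted as unsuited to multiple player characters.
; A third finds a path to that player synchronously and draws debug spheres at each path point.
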(event EventBeginPlay)

(fn ConstructionScript)